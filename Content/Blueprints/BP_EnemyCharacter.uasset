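; BP_EnemyCharacter is an enemy character that takes damage and awards score when killed.
; Capsule overlaps or hits with the combat player start contact through the game mode, and overlap end closes it.
; ReceiveDamage reduces life points, then at zero or below adds score through the cached game instance and unregisters the enemy from the game mode.
; MakeDamage is an empty stub, and MyGameMode is not assigned here.
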(event `self.ReceiveBeginPlay`
  (bind _asbp_game_instance (cast `/Game/Blueprints/BP_GameInstance` (`GameplayStatics.GetGameInstance`)))
  (set `self.MyGameInstance` _asbp_game_instance))

(event `self.CapsuleComponent.OnComponentBeginOverlap`
  (params (OverlappedComponent :type "PrimitiveComponent Object Reference") (OtherActor :type "Actor Object Reference") (OtherComp :type "PrimitiveComponent Object Reference") (OtherBodyIndex :type Integer) (bFromSweep :type Boolean) (SweepResult :type "HitResult Structure (by ref)"))
  (cast `/Game/Blueprints/BP_CombatPlayerCharacter` (stale `self.CapsuleComponent.OnComponentHit` OtherActor) :!label _label)
  (`/Game/Blueprints/BP_GameMode.StartContactWithEnemy` (`self.MyGameMode`) self))

(event `self.CapsuleComponent.OnComponentHit`
  (params (HitComponent :type "PrimitiveComponent Object Reference") (OtherActor :type "Actor Object Reference") (OtherComp :type "PrimitiveComponent Object Reference") (NormalImpulse :type "Vector Structure") (Hit :type "HitResult Structure (by ref)"))
  (goto _label))

(event `self.CapsuleComponent.OnComponentEndOverlap`
  (params (OverlappedComponent :type "PrimitiveComponent Object Reference") (OtherActor :type "Actor Object Reference") (OtherComp :type "PrimitiveComponent Object Reference") (OtherBodyIndex :type Integer))
  (cast `/Game/Blueprints/BP_CombatPlayerCharacter` OtherActor)
  (`/Game/Blueprints/BP_GameMode.EndContactWithCurrentEnemy` (`self.MyGameMode`) self))

(fn `MakeDamage`)

(fn `ReceiveDamage`
  (params (Damage :type "Float (double-precision)"))
  (bind _output_get (set `self.LifePoints` (- (`self.LifePoints`) Damage)))
  (if (<= _output_get 0.0)
    (`/Game/Blueprints/BP_GameInstance.AddPointsToScore` (`self.MyGameInstance`) (`self.KilledScorePoints`))
    (`/Game/Blueprints/BP_GameMode.UnregisterEnemy` (`self.MyGameMode`) self)))

(fn `UserConstructionScript`)