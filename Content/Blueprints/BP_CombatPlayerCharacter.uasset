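; Combat player character that teleports to target locations and takes damage against life points stored in the game instance.
; BeginPlay caches the game instance and game mode; ReceiveDamage notifies the game mode when life runs out.
; UpdateAttack is a state machine that checks proximity to the current enemy, deals damage, scores points and returns to idle, but its EventGraph call is disconnected and Tick is empty.
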(event `self.ReceiveBeginPlay`
  (bind _asbp_game_instance (cast `/Game/Blueprints/BP_GameInstance` (`GameplayStatics.GetGameInstance`)))
  (set `self.MyGameInstance` _asbp_game_instance)
  (bind _asbp_game_mode (cast `/Game/Blueprints/BP_GameMode` (`GameplayStatics.GetGameMode`)))
  (set `self.MyGameMode` _asbp_game_mode))

(event `self.ReceiveTick`
  (params (DeltaSeconds :type "Float (single-precision)")))

(fn `MoveToLocation`
  (params (TargetLocation :type "Vector Structure"))
  (locals (DirectionToTarget :type "Vector Structure"))
  (`self.K2_TeleportTo` TargetLocation))

(fn `ReceiveDamage`
  (params (Damage :type "Float (double-precision)"))
  (bind _mygameinstance (`self.MyGameInstance`))
  (set `/Game/Blueprints/BP_GameInstance.CurrentLifePoints` (- (`/Game/Blueprints/BP_GameInstance.CurrentLifePoints` _mygameinstance) Damage) _mygameinstance)
  (if (not (> (`/Game/Blueprints/BP_GameInstance.CurrentLifePoints` (`self.MyGameInstance`)) 0.0))
    (`/Game/Blueprints/BP_GameMode.Player Dies` (`self.MyGameMode`))))

(fn `UpdateAttack`
  (bind _currentenemy (`/Game/Blueprints/BP_GameMode.CurrentEnemy` (`self.MyGameMode`)))
  (bind _currentenemy_2 (`/Game/Blueprints/BP_GameMode.CurrentEnemy` (`self.MyGameMode`)))
  (switch `/Game/Blueprints/E_PlayerState` (`self.CurrentState`)
    (:`NewEnumerator1`
      (`/Engine/EditorBlueprintResources/StandardMacros.IsValid` _currentenemy_2
        (:`Is Valid`
          (if (<= (`KismetMathLibrary.Vector_Distance` (`self.K2_GetActorLocation` _currentenemy_2) (`self.K2_GetActorLocation`)) 0.1)
            (set `self.CurrentState` "NewEnumerator2")
            (`self.K2_SetActorLocation` (`KismetMathLibrary.VInterpTo_Constant` (`self.K2_GetActorLocation`) (`self.K2_GetActorLocation` _currentenemy_2) (`GameplayStatics.GetWorldDeltaSeconds`) (`self.Speed`)))))))
    (:`NewEnumerator2`
      (`/Engine/EditorBlueprintResources/StandardMacros.IsValid` _currentenemy
        (:`Is Valid`
          (bind _points (`/Game/Blueprints/BP_EnemyCharacter.ReceiveDamage` _currentenemy (`self.Damage`)))
          (`/Game/Blueprints/BP_GameInstance.AddPointsToScore` (`self.MyGameInstance`) _points)
          (set `self.CurrentState` "NewEnumerator0")
          (set `self.IsBlockMovement` false))))))

(fn `UserConstructionScript`)