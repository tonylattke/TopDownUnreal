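; Enemy manager that coordinates which enemies chase the player, based on the player's current state.
; BeginPlay caches the game mode and player; every Tick branches on Idle or Attacking.
; Idle promotes one waiting enemy when none are chasing, while Attacking promotes another each tick when a chaser already exists.
; UpdateChaser, not called here, makes a given enemy the sole chaser, skipping certain states.
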(event `self.ReceiveBeginPlay`
  (bind _asbp_game_mode (cast `/Game/Blueprints/BP_GameMode` (`GameplayStatics.GetGameMode`)))
  (bind _output_get (set `self.MyGameMode` _asbp_game_mode))
  (set `self.Player Character` (`/Game/Blueprints/BP_GameMode.PlayerCharacter` _output_get)))

(event `self.ReceiveTick`
  (params (DeltaSeconds :type "Float (single-precision)"))
  (`self.Update`))

(fn `HandlePlayerAttack`
  (locals (ChaseEnemy :type "/Game/Blueprints/BP_EnemyCharacter Object Reference"))
  (if (not (`/Game/Blueprints/BP_GameMode.ThereIsAtLeastOneEnemyIn` (`self.MyGameMode`) "NewEnumerator1"))
    (return)
    (else
      (bind _result (`/Game/Blueprints/BP_GameMode.GetOneEnemyInState` (`self.MyGameMode`) "NewEnumerator0"))
      (set `local.ChaseEnemy` _result)
      (`/Engine/EditorBlueprintResources/StandardMacros.IsValid` _result
        (:`Is Valid`
          (set `/Game/Blueprints/BP_EnemyCharacter.CurrentState` "NewEnumerator1" (`local.ChaseEnemy`)))))))

(fn `HandlePlayerIdle`
  (locals (ChaseEnemy :type "/Game/Blueprints/BP_EnemyCharacter Object Reference"))
  (if (`/Game/Blueprints/BP_GameMode.ThereIsAtLeastOneEnemyIn` (`self.MyGameMode`) "NewEnumerator1")
    (return)
    (else
      (bind _result (`/Game/Blueprints/BP_GameMode.GetOneEnemyInState` (`self.MyGameMode`) "NewEnumerator0"))
      (set `local.ChaseEnemy` _result)
      (`/Engine/EditorBlueprintResources/StandardMacros.IsValid` _result
        (:`Is Valid`
          (set `/Game/Blueprints/BP_EnemyCharacter.CurrentState` "NewEnumerator1" (`local.ChaseEnemy`)))))))

(fn `Update`
  (switch `/Game/Blueprints/E_PlayerState` (`/Game/Blueprints/BP_CombatPlayerCharacter.CurrentState` (`self.Player Character`))
    (:`NewEnumerator0`
      (`self.HandlePlayerIdle`))
    (:`NewEnumerator2`
      (`self.HandlePlayerAttack`))))

(fn `UpdateChaser`
  (params (Enemy :type "/Game/Blueprints/BP_EnemyCharacter Object Reference"))
  (if (`|EnumEquality` (`/Game/Blueprints/BP_EnemyCharacter.CurrentState` Enemy) "NewEnumerator2")
    (return)
    (else
      (for _array_element (`/Game/Blueprints/BP_GameMode.Enemies` (`self.MyGameMode`))
        (if (and (!= _array_element (`local.Enemy`)) (not (`|EnumEquality` (`/Game/Blueprints/BP_EnemyCharacter.CurrentState` _array_element) "NewEnumerator3")))
          (set `/Game/Blueprints/BP_EnemyCharacter.CurrentState` "NewEnumerator0" _array_element)))
      (set `/Game/Blueprints/BP_EnemyCharacter.CurrentState` "NewEnumerator1" Enemy))))

(fn `UserConstructionScript`)