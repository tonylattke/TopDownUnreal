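; Game mode that runs combat levels, tracking enemies, the player's current target, the hit counter and score.
; On BeginPlay it sets up the HUD and, if BP_LevelHandler reports Combat, spawns BP_EnemyManagerAI and links all enemies to itself.
; Combat Tick drops out-of-range targets, banks the counter into the GameInstance score when its timer expires, and checks for victory.
; All enemies dead or player death opens the score level.
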(event `self.ReceiveBeginPlay`
  (`|ExecutionSequence`
    (:`then_0`
      (`self.Initialize HUD`)
      (bind _asbp_game_instance (cast `/Game/Blueprints/BP_GameInstance` (`GameplayStatics.GetGameInstance`)))
      (set `self.MyGameInstance` _asbp_game_instance)
      (bind _returnvalue (`GameplayStatics.GetActorOfClass` "/Game/Blueprints/BP_LevelHandler.BP_LevelHandler_C"))
      (bind _output_get (set `self.LevelHandler` _returnvalue))
      (set `self.LevelType` (`/Game/Blueprints/BP_LevelHandler.CurrentLevelType` _output_get)))
    (:`then_2`
      (switch `/Game/Blueprints/E_LevelType` (`self.LevelType`)
        (:`NewEnumerator0`
          (bind _returnvalue_2 (`|SpawnActorFromClass` "/Game/Blueprints/BP_EnemyManagerAI.BP_EnemyManagerAI_C" (`KismetMathLibrary.MakeTransform` (0.0 0.0 0.0)) "Undefined" "MultiplyWithRoot" null null))
          (set `self.EnemyManagerAI` _returnvalue_2)
          (`self.InitializeCombatLevel`))))))

(event `self.ReceiveTick`
  (params (DeltaSeconds :type "Float (single-precision)"))
  (switch `/Game/Blueprints/E_LevelType` (`self.LevelType`)
    (:`NewEnumerator0`
      (`self.CheckIfEnemyStillOnRange`)
      (`self.UpdateCounterTimer`)
      (`self.CheckWin`))))

(fn `AddAttackCounter`
  (`/Game/Blueprints/BP_GameInstance.AddCounterPoint` (`self.MyGameInstance`))
  (`self.ResetCounterTimer`))

(fn `AreAllEnemiesDead`
  (returns (Result :type Boolean))
  (for _array_element (`self.Enemies`)
    (if (not (`|EnumEquality` (`/Game/Blueprints/BP_EnemyCharacter.CurrentState` _array_element) "NewEnumerator4"))
      (return false)))
  (return true))

(fn `CheckIfEnemyStillOnRange`
  (`/Engine/EditorBlueprintResources/StandardMacros.IsValid` (`self.CurrentEnemy`)
    (:`Is Valid`
      (if (> (`KismetMathLibrary.Vector_Distance` (`self.K2_GetActorLocation` (`self.CurrentEnemy`)) (`self.K2_GetActorLocation` (`self.PlayerCharacter`))) (`self.RangeEnemy`))
        (set `self.CurrentEnemy` null)))))

(fn `CheckWin`
  (bind _mygameinstance (`self.MyGameInstance`))
  (if (`self.AreAllEnemiesDead`)
    (`/Game/Blueprints/BP_GameInstance.AddPointsToScore` _mygameinstance (`/Game/Blueprints/BP_GameInstance.EvaluateCounterBonus` _mygameinstance))
    (`GameplayStatics.OpenLevel` "L_Score")))

(fn `DeleteEnemy`
  (params (EnemyToDelete :type "/Game/Blueprints/BP_EnemyCharacter Object Reference (by ref)"))
  (`KismetArrayLibrary.Array_RemoveItem` (`self.Enemies`) EnemyToDelete))

(fn `EndContactWithCurrentEnemy`
  (params (ContactedEnemy :type "/Game/Blueprints/BP_EnemyCharacter Object Reference"))
  (if (== ContactedEnemy (`self.CurrentEnemy`))
    (set `self.CurrentEnemy` null)
    (`KismetSystemLibrary.PrintString` "Stop" true true (struct :`R` 1.0 :`G` 0.001 :`A` 1.0))))

(fn `FailCounter`
  (bind _mygameinstance (`self.MyGameInstance`))
  (set `self.CounterResetTimer` 0.0)
  (bind _lastcounter (`/Game/Blueprints/BP_GameInstance.DeleteCounter` _mygameinstance))
  (`/Game/Blueprints/BP_GameInstance.AddPointsToScore` _mygameinstance (* _lastcounter (`/Game/Blueprints/BP_GameInstance.GetKilledEnemies` _mygameinstance)))
  (set `/Game/Blueprints/BP_GameInstance.AmountOfEnemyKilled` 0 _mygameinstance)
  (set `self.CurrentEnemy` null))

(fn `GetOneEnemyInState`
  (params (State :type "/Game/Blueprints/E_EnemyState Enum" :default "NewEnumerator0"))
  (returns (Result :type "/Game/Blueprints/BP_EnemyCharacter Object Reference"))
  (for _array_element (`self.Enemies`)
    (if (`|EnumEquality` (`/Game/Blueprints/BP_EnemyCharacter.CurrentState` _array_element) State)
      (return _array_element)))
  (return null))

(fn `InitialazeEnemies`
  (bind _outactors (`GameplayStatics.GetAllActorsOfClass` "/Game/Blueprints/BP_EnemyCharacter.BP_EnemyCharacter_C"))
  (set `self.Enemies` _outactors)
  (for _array_element _outactors
    (set `/Game/Blueprints/BP_EnemyCharacter.MyGameMode` self _array_element)))

(fn `Initialize HUD`
  (bind _asbp_hud (cast `/Game/Blueprints/BP_HUD` (`PlayerController.GetHUD` (`GameplayStatics.GetPlayerController` 0))))
  (set `self.HUD` _asbp_hud)
  (`/Game/Blueprints/BP_HUD.Initialize` _asbp_hud))

(fn `InitializeCombatLevel`
  (`|ExecutionSequence`
    (:`then_0`
      (bind _asbp_combat_player_character (cast `/Game/Blueprints/BP_CombatPlayerCharacter` (`GameplayStatics.GetPlayerPawn` 0)))
      (set `self.PlayerCharacter` _asbp_combat_player_character))
    (:`then_1`
      (`self.InitialazeEnemies`))
    (:`then_2`
      (`/Game/Blueprints/BP_HUD.ShowInGameUI` (`self.HUD`)))))

(fn `Player Dies`
  (`GameplayStatics.OpenLevel` "L_Score"))

(fn `ResetCounterTimer`
  (set `self.CounterResetTimer` (`self.CounterResetTimerMax`)))

(fn `Set New Enemy`
  (params (NewEnemy :type "/Game/Blueprints/BP_EnemyCharacter Object Reference"))
  (set `self.CurrentEnemy` NewEnemy))

(fn `SetEnemyAsAttacker`
  (params (Enemy :type "/Game/Blueprints/BP_EnemyCharacter Object Reference"))
  (`/Game/Blueprints/BP_GameInstance.AddCounterPoint` (`self.MyGameInstance`))
  (`self.ResetCounterTimer`)
  (`/Game/Blueprints/BP_EnemyManagerAI.UpdateChaser` (`self.EnemyManagerAI`) Enemy))

(fn `StartContactWithEnemy`
  (params (NewEnemy :type "/Game/Blueprints/BP_EnemyCharacter Object Reference"))
  (bind _currentenemy (`self.CurrentEnemy`))
  (`/Engine/EditorBlueprintResources/StandardMacros.IsValid` _currentenemy
    (:`Is Valid`
      (if (not (== NewEnemy _currentenemy))
        (`self.Set New Enemy` NewEnemy)))
    (:`Is Not Valid`
      (`self.Set New Enemy` NewEnemy))))

(fn `ThereIsAtLeastOneEnemyIn`
  (params (State :type "/Game/Blueprints/E_EnemyState Enum" :default "NewEnumerator0"))
  (returns (Result :type Boolean))
  (for _array_element (`self.Enemies`)
    (if (`|EnumEquality` (`/Game/Blueprints/BP_EnemyCharacter.CurrentState` _array_element) State)
      (return true)))
  (return false))

(fn `UnregisterEnemy`
  (params (Enemy :type "/Game/Blueprints/BP_EnemyCharacter Object Reference"))
  (`|ExecutionSequence`
    (:`then_0`
      (if (== Enemy (`self.CurrentEnemy`))
        (set `self.CurrentEnemy` null)))
    (:`then_1`
      (`KismetArrayLibrary.Array_RemoveItem` (`self.Enemies`) Enemy)
      (`self.K2_DestroyActor` Enemy))))

(fn `UpdateCounterTimer`
  (bind _mygameinstance (`self.MyGameInstance`))
  (bind _currentcounter (`/Game/Blueprints/BP_GameInstance.CurrentCounter` _mygameinstance))
  (if (and (> _currentcounter 0) (> (`self.CounterResetTimer`) 0.0))
    (set `self.CounterResetTimer` (- (`self.CounterResetTimer`) (* (`GameplayStatics.GetWorldDeltaSeconds`) (`self.CounterResetSpeed`))))
    (else
      (`/Game/Blueprints/BP_GameInstance.AddPointsToScore` (`self.MyGameInstance`) _currentcounter)
      (set `/Game/Blueprints/BP_GameInstance.CurrentCounter` 0 _mygameinstance))))

(fn `UserConstructionScript`)